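; BP_BooSpawnCube is an interactable cube that releases a Boo enemy and makes the level's keys available.
; On Interact, it hides itself, switches its text to the alive message, spawns BP_Boo just above its location and activates and reveals every BP_Key actor.
; Its Reset function shows the cube again and restores the inactive text, leaving the spawned Boo and keys untouched.
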(event EventBeginPlay)

(event Collision|EventActorBeginOverlap
  (params (OtherActor :type Actor%20Object%20Reference)))

(event EventTick
  (params (DeltaSeconds :type Float%20%28single-precision%29)))

(event EventInteract
  ;[1 1 1] Interact Interface Override
  (Rendering|Components|TextRender|SetText (Variables|Default|GetTextRender) (Variables|Default|GetBoo%20Alive%20Text))
  (Rendering|SetVisibility (Variables|Default|GetCube) false false)
  (Game|SpawnActorfromClass "/Game/Blueprints/BP_Boo.BP_Boo_C" (Math|Conversions|ToTransform(Vector) (+ (Transformation|GetActorLocation) "0,0,100.000000")) "Undefined" 0 0)
  (bind _outactors (Actor|GetAllActorsOfClass "/Game/Blueprints/BP_Key.BP_Key_C"))
  (for _array_element _outactors
    (Variables|/Game/Blueprints/BP_Key.BP_Key_C|SetActive _array_element true)
    (Rendering|SetVisibility (Variables|/Game/Blueprints/BP_Key.BP_Key_C|GetCube _array_element) true false)))

(fn ConstructionScript)

(fn Reset
  (Rendering|SetVisibility (Variables|Default|GetCube) true false)
  (Rendering|Components|TextRender|SetText (Variables|Default|GetTextRender) (LocalVariables|GetBoo%20Inactive%20Text)))