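; BP_redCube is an interactable actor that switches a particle system and an audio effect on and off.
; It implements an Interact interface event that checks an Active flag, activates or deactivates both components together, then flips the flag.
; All behavior runs from that event, as BeginPlay, overlap, Tick and the construction script are empty.
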(event EventBeginPlay)

(event Collision|EventActorBeginOverlap
  (params (OtherActor :type Actor%20Object%20Reference)))

(event EventTick
  (params (DeltaSeconds :type Float%20%28single-precision%29)))

(event EventInteract
  ;[1 1 1] Interact Interface Override
  (if (Variables|Default|GetActive)
    (Components|Activation|Deactivate (Variables|Default|GetParticleSystem))
    (Components|Activation|Deactivate (Variables|Default|GetAudio))
    (Variables|Default|SetActive false)
    (else
      (Components|Activation|Activate (Variables|Default|GetParticleSystem) false)
      (Components|Activation|Activate (Variables|Default|GetAudio) false)
      (Variables|Default|SetActive true))))

(fn ConstructionScript)