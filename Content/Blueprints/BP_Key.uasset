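; BP_Key is an interactable key pickup that gives the player character a key.
; Its cube mesh is hidden on BeginPlay, and the Interact interface event only responds while the Active flag is set.
; Interact calls AddKey on every BP_Character in the level, plays a half-second particle burst, then hides the cube.
; Nothing here sets or clears Active or makes the cube visible.
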(event EventBeginPlay
  ;[1 1 1] Begin Play
  (Rendering|SetVisibility (Variables|Default|GetCube) false false))

(event EventInteract
  ;[1 1 1] Interact Interface Override
  (if (Variables|Default|GetActive)
    (bind _outactors (Actor|GetAllActorsOfClass "/Game/Blueprints/BP_Character.BP_Character_C"))
    (for _array_element _outactors
      (Default|AddKey _array_element))
    (Components|Activation|Activate (Variables|Default|GetParticleSystem) false)
    (Utilities|FlowControl|Delay 0.5)
    (Components|Activation|Deactivate (Variables|Default|GetParticleSystem))
    (Rendering|SetVisibility (Variables|Default|GetCube) false false)))

(fn ConstructionScript)