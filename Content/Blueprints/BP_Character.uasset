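; BP_Character is a player character that looks around with the mouse, teleports, interacts by gaze and tracks collected keys.
; Each tick a camera line trace stores the hit location and any actor implementing BP_InteractInterface.
; Click messages that actor, or otherwise teleports to just above the hit point.
; AddKey counts keys; at the target it records a Boo's hit count as score, destroys all Boos, resets spawn cubes and key count, and prints the score.
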(event Custom|GazeCheck
  (bind _camera (Variables|Default|GetCamera))
  (bind _returnvalue (Transformation|GetWorldLocation _camera))
  ;[1 1 1] Gaze check
  (bind _outhit (Collision|LineTraceByChannel _returnvalue (+ _returnvalue (* (Math|Vector|GetForwardVector _camera) 2000)) "TraceTypeQuery1" false 0 "ForOneFrame"))
  (Variables|Default|SetViewHitLocation (.Location (Collision|BreakHitResult _outhit)))
  (if (Utilities|DoesObjectImplementInterface (.HitActor (Collision|BreakHitResult _outhit)) "/Game/Blueprints/BP_InteractInterface.BP_InteractInterface_C")
    (Variables|Default|SetinteractingActor (.HitActor (Collision|BreakHitResult _outhit)))
    (else
      (Variables|Default|SetinteractingActor 0))))

(event EventTick
  (params (DeltaSeconds :type Float%20%28single-precision%29))
  (CallFunction|GazeCheck))

(event Input|ActionEvents|InputActionClick
  (params (Key :type Key%20Structure :default "None"))
  (bind _interactingactor (Variables|Default|GetinteractingActor))
  ;[1 1 1] Input
  (:Pressed
    (Utilities|IsValid _interactingactor
      (:Is%20Valid
        (Class|BPInteractInterface|Interact(Message) _interactingactor))
      (:Is%20Not%20Valid
        (Transformation|Teleport (+ (Variables|Default|GetViewHitLocation) "0,0,88.000000") "0, 0, 0")))))

(event Input|AxisEvents|InputAxismouseX
  (params (AxisValue :type Float%20%28single-precision%29))
  ;[1 1 1] Input
  (Pawn|Input|AddControllerYawInput AxisValue))

(event Input|AxisEvents|InputAxismouseY
  (params (AxisValue :type Float%20%28single-precision%29))
  ;[1 1 1] Input
  (Pawn|Input|AddControllerPitchInput AxisValue))

(fn ConstructionScript)

(fn AddKey
  ;[1 1 1] Add Key Function
  (bind _result (Math|Integer|IncrementInt (Variables|Default|GetKeysFound))
    (:%20%20
      (if (== _result (Variables|Default|GetNum%20Keys)) ; Continue if all keys found
        (Development|PrintString (Utilities|String|Append "Number of Keys: " (Utilities|String|ToString(Integer) (Variables|Default|GetKeysFound))) true true "(R=1.000000,G=0.983694,B=0.000000,A=1.000000)" 2.0 "11")
        (bind _outactors (Actor|GetAllActorsOfClass "/Game/Blueprints/BP_Boo.BP_Boo_C")) ; Kill all boos
        (for _array_element _outactors
          (Variables|Default|SetScore (Variables|/Game/Blueprints/BP_Boo.BP_Boo_C|GetHit%20Count _array_element))
          (Actor|DestroyActor _array_element))
        (bind _outactors_2 (Actor|GetAllActorsOfClass "/Game/Blueprints/BP_BooSpawnCube.BP_BooSpawnCube_C")) ; Bring back the spawn block
        (for _array_element_2 _outactors_2
          (Default|Reset _array_element_2))
        (Variables|Default|SetKeysFound 0) ; Reset Key Count
        (Development|PrintString (Utilities|String|Append "Final Score: " (Utilities|String|ToString(Integer) (Variables|Default|GetScore))) true true "(R=1.000000,G=0.935926,B=0.000000,A=1.000000)" 1e+01 "11")))))