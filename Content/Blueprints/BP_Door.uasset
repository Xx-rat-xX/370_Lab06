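; BP_Door is an interactable sliding door that opens and closes through the Interact interface event.
; Interact plays the DoorDriver timeline when DoorClosed is true and reverses it otherwise.
; The timeline's Driver track lerps the DoorWay component's relative location between DoorStart and DoorStop without sweeping.
; DoorClosed flips only when the timeline finishes, so an interaction mid-motion does not change direction.
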(event EventBeginPlay)

(event Collision|EventActorBeginOverlap
  (params (OtherActor :type Actor%20Object%20Reference)))

(event EventTick
  (params (DeltaSeconds :type Float%20%28single-precision%29)))

(event EventInteract
  ;[1 1 1] Interactive Interface Override
  (if (Variables|Default|GetDoorClosed)
    (bind _driver (Timeline|Door%20Driver Play)
      (:Update
        (Transformation|SetRelativeLocation (Variables|Default|GetDoorWay) (Math|Vector|Lerp(Vector) (Variables|DoorSetup|GetDoorStart) (Variables|DoorSetup|GetDoorStop) _driver) false false))
      (:Finished
        (Variables|Default|SetDoorClosed (not (Variables|Default|GetDoorClosed)))))
    (else
      (Timeline|Door%20Driver Reverse))))

(fn ConstructionScript)