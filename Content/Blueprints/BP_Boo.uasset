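; BP_Boo is a Boo-style ghost enemy that creeps toward the player only while off screen.
; When recently rendered, it holds still and a timeline drives its dynamic material's opacity; unseen, it reverses the fade and lerps toward the pawn, facing it.
; Proximity prints a warning, then a hit that costs score and teleports it to a random point around the world origin's positive octant.
; Interact adds score and also teleports it.
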(event EventTick
  (params (DeltaSeconds :type Float%20%28single-precision%29))
  (bind _returnvalue (Game|Player|GetPlayerPawn 0))
  (bind _returnvalue_2 (Transformation|GetActorLocation))
  (bind _returnvalue_3 (Transformation|GetActorLocation _returnvalue))
  (bind _returnvalue_4 (Math|Vector|Lerp(Vector) _returnvalue_2 _returnvalue_3 0.03))
  (bind _returnvalue_5 (Math|Vector|Distance(Vector) _returnvalue_4 _returnvalue_3))
  ;[1 1 1] Tick
  (if (Class|Actor|WasRecentlyRendered 0.2)
    (bind _translucency (Timeline|Timeline%20Translucent%20Driver Play)
      (:Update
        (Rendering|Material|SetScalarParameterValue (Variables|Default|GetTranslucent%20Material%20Instance) "OpacityAmount" _translucency :!class /Script/Engine.MaterialInstanceDynamic)))
    (else
      (Transformation|SetActorLocation _returnvalue_4 false false)
      (Transformation|SetActorRotation (Math|Rotator|FindLookatRotation _returnvalue_4 _returnvalue_3))
      (if (< _returnvalue_5 (Variables|Default|GetBooProxWarn))
        (Development|PrintString "BOO IS NEAR" true true "(R=1.000000,G=0.441736,B=0.000000,A=1.000000)" 1.0 "1")
        (if (< _returnvalue_5 (Variables|Default|GetBooProxHit))
          (Development|PrintString "YOU WERE HIT!!!" true true "(R=1.000000,G=0.000000,B=0.012353,A=1.000000)" 2.0 "1")
          (CallFunction|SendtoNewLocation)
          (Variables|Default|SetHit%20Count (- (Variables|Default|GetHit%20Count) 5))
          (Timeline|Timeline%20Translucent%20Driver Reverse)
          (else
            (Timeline|Timeline%20Translucent%20Driver Reverse)))
        (else
          (Timeline|Timeline%20Translucent%20Driver Reverse))))))

(event EventBeginPlay
  ;[1 1 1] Begin Play
  (bind _returnvalue (Rendering|Material|CreateDynamicMaterialInstance (Variables|Default|GetSphere) 0 "/Game/MAterials/M_boo_Inst.M_boo_Inst" "None" :!class /Script/Engine.PrimitiveComponent))
  (Variables|Default|SetTranslucent%20Material%20Instance _returnvalue))

(event EventInteract
  ;[1 1 1] Hit Interface Override
  (bind _result (Math|Integer|IncrementInt (Variables|Default|GetHit%20Count))
    (:%20%20
      (Development|PrintString (Utilities|String|Append "Your Score: " (Utilities|String|ToString(Integer) _result)) true true "(R=0.000000,G=0.660000,B=1.000000,A=1.000000)" 2.0 "10")
      (CallFunction|SendtoNewLocation))))

(fn ConstructionScript)

(fn SendtoNewLocation
  (Transformation|SetActorLocation (* (Math|Vector|VectorGetAbs (Math|Random|RandomUnitVector)) (Variables|Default|GetTeleport%20Radius)) false false))